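; BP_ConfigController is the player controller for a car configurator, acting as the bridge between the HUD and the game mode.
; On BeginPlay it creates the HUD widget with UI-only input and a visible cursor, then caches the ConfigGameMode.
; HUD events for previous/next car and colour changes are forwarded to the game mode.
; The game mode's new-car event flows back to the HUD to update the displayed stats.
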(event Custom|NewCar
  (params (NewCar :type Car%20Info%20Struct%20Structure))
  (bind _hud (Variables|Default|GetHud))
  ;[1 1 1] When the Game mode changes car, tell the HUD to update all the stats
  (Utilities|IsValid _hud
    (:Is%20Valid
      (Default|UpdateCar _hud NewCar))))

(event Custom|RequestNewCar
  (params (Previous? :type Boolean))
  (bind _configgamemode (Variables|Default|GetConfigGameMode))
  ;[1 1 1] HUD buttons have been pressed to request a new car, ask the Game Mode to do so
  (if Previous?
    (Default|PrevCar _configgamemode)
    (else
      (Default|NextCar _configgamemode))))

(event Custom|UpdateCarColour
  (params (NewColourTexture :type Texture%202D%20Object%20Reference))
  ;[1 1 1] HUD has asked to change the colour, so reflect this on the car via the game mode
  (Default|ChangeColour (Variables|Default|GetConfigGameMode) NewColourTexture))

(event EventBeginPlay
  (Utilities|FlowControl|Sequence
    (:then_0
      ;[1 1 1] Create the HUD Widget and store it for later use
      (bind _returnvalue (UserInterface|CreateWidget "/Game/blueprints/widgets/WB_Hud.WB_Hud_C"))
      (bind _output_get (Variables|Default|SetHud _returnvalue))
      (UserInterface|Viewport|AddtoViewport _output_get 0)
      (Input|SetInputModeUIOnly self (Variables|Default|GetHud) "DoNotLock")
      (Variables|Default|SetbShowMouseCursor true))
    (:then_1
      ;[1 1 1] Store the correct Game mode for later use
      (bind _asconfig_game_mode (Utilities|Casting|CastToConfigGameMode (Game|GetGameMode)))
      (Variables|Default|SetConfigGameMode _asconfig_game_mode))
    (:then_2
      ;[1 1 1] When the Game mode changes car, tell the HUD to update all the stats
      (EventDispatchers|BindEventtoUpdateNewCar (Variables|Default|GetConfigGameMode) (delegate Custom|NewCar)))
    (:then_3
      ;[1 1 1] HUD buttons have been pressed to request a new car, ask the Game Mode to do so
      (EventDispatchers|BindEventtoObtainNewCar (Variables|Default|GetHud) (delegate Custom|RequestNewCar)))
    (:then_4
      ;[1 1 1] HUD has asked to change the colour, so reflect this on the car via the game mode
      (EventDispatchers|BindEventtoColourHasChanged (Variables|Default|GetHud) (delegate Custom|UpdateCarColour)))))

(fn ConstructionScript)