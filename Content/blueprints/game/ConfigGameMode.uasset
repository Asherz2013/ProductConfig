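; ConfigGameMode is the game mode for a car configurator, tracking the current car and broadcasting car and colour changes.
; On PostLogin it caches the Cars data table row names, then after a short delay shows the current car.
; NextCar and PrevCar wrap the index around the list, and SetNewCar sends that row through the UpdateNewCar dispatcher.
; ChangeColour relays the chosen colour through the UpdateColour dispatcher.
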(event Custom|ChangeColour
  (params (NewColour :type Texture%202D%20Object%20Reference))
  ;[1 1 1] Dispatch that a colour has changed
  (Default|CallUpdateColour NewColour))

(event Custom|NextCar
  ;[1 1 1] New car was requested, loop round the array and setup the new car.
  (Variables|Default|SetCurrent_car (Math|Integer|%(Integer) (+ (Variables|Default|GetCurrent_car) 1) (Variables|Default|GetMax_cars)))
  (CallFunction|SetNewCar))

(event Custom|PrevCar
  ;[1 1 1] New car was requested, loop backwards but make sure we don't go out the array index and setup the new car.
  (if (<= (- (Variables|Default|GetCurrent_car) 1) -1)
    (Variables|Default|SetCurrent_car (- (Variables|Default|GetMax_cars) 1))
    (else
      (Variables|Default|SetCurrent_car (- (Variables|Default|GetCurrent_car) 1))))
  (CallFunction|SetNewCar))

(event EventPostLogin
  (params (NewPlayer :type Player%20Controller%20Object%20Reference))
  ;[1 1 1] When the player logs in, store all the Car information and tell the relevant components to update a new car has been shown
  (bind _outrownames (DataTable|GetDataTableRowNames "/Game/blueprints/assets/cars.cars"))
  (bind _output_get (Variables|Default|SetCars _outrownames))
  (Variables|Default|SetMax_cars (Utilities|Array|Length _output_get))
  (Utilities|FlowControl|Delay 0.2)
  (CallFunction|SetNewCar))

(fn ConstructionScript)

(fn SetNewCar
  (bind _returnvalue (Utilities|GetDataTableRow "/Game/blueprints/assets/cars.cars" (Utilities|Array|Get(acopy) (Variables|Default|GetCars) (Variables|Default|GetCurrent_car)))
    (:then
      (Default|CallUpdateNewCar _returnvalue))))