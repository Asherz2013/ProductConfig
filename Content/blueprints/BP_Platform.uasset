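; BP_Platform is a display platform that shows the selected car model and body colour in a car configurator.
; On BeginPlay it binds handlers to the ConfigGameMode's new-car and colour-update events.
; A new car swaps the skeletal mesh and creates a dynamic material instance on its first material slot.
; Colour changes are applied to that instance by setting a texture parameter rather than a colour value.
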(event Custom|NewCar
  (params (NewCar :type Car%20Info%20Struct%20Structure))
  ;[1 1 1] When the game mode requests a new car to be shown, update the model and setup a Material Instance to help with changing colour
  (Class|SkinnedMeshComponent|SetSkeletalMesh (Variables|Default|GetCar) (Utilities|Struct|Breakcar_Info_struct NewCar) true)
  (bind _returnvalue (Rendering|Material|CreateDynamicMaterialInstance (Variables|Default|GetCar) 0 "/Game/blueprints/assets/materials/ColorVar1_Material.ColorVar1_Material" "None" :!class /Script/Engine.PrimitiveComponent))
  (Variables|Default|SetBodyColour _returnvalue))

(event Custom|NewColour
  (params (NewColour :type Texture%202D%20Object%20Reference))
  ;[1 1 1] When the game mode requests a new Colour, change it on the Intance
  (Rendering|Material|SetTextureParameterValue (Variables|Default|GetBodyColour) "Param" NewColour))

(event EventBeginPlay
  (bind _asconfig_game_mode (Utilities|Casting|CastToConfigGameMode (Game|GetGameMode)))
  (Utilities|FlowControl|Sequence
    (:then_0
      ;[1 1 1] When the game mode requests a new car to be shown, update the model and setup a Material Instance to help with changing colour
      (EventDispatchers|BindEventtoUpdateNewCar _asconfig_game_mode (delegate Custom|NewCar)))
    (:then_1
      ;[1 1 1] When the game mode requests a new Colour, change it on the Intance
      (EventDispatchers|BindEventtoUpdateColour _asconfig_game_mode (delegate Custom|NewColour)))))

(fn ConstructionScript)